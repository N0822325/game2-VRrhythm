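; ScoreBP is a score display actor that keeps a running Score and shows it on a TextRender component.
; Two events, incscore and decscore, raise or lower Score by one and immediately write the new value to the text, with no bounds check.
; It has no active BeginPlay, overlap or Tick logic, so the score and text change only when those events are called.
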(event `inc score`
  (bind _score (`self.Score`))
  (`/Engine/EditorBlueprintResources/StandardMacros.IncrementInt` _score
    (:`  `
      (`TextRenderComponent.K2_SetText` (`self.TextRender`) (`KismetTextLibrary.Conv_IntToText` _score)))))

(event `dec score`
  (bind _score (`self.Score`))
  (`/Engine/EditorBlueprintResources/StandardMacros.DecrementInt` _score
    (:`  `
      (`TextRenderComponent.K2_SetText` (`self.TextRender`) (`KismetTextLibrary.Conv_IntToText` _score)))))

(fn `UserConstructionScript`)